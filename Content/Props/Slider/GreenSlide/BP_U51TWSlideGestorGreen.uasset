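; Manager actor for the green slide, which carries a Character on a Cart platform along a spline.
; On BeginPlay it attaches the Character and starts the spline move with increasing speed, then destroys the Cart and itself on completion.
; Tick keeps the Character's position updated on the platform.
; Each step branches on authority, calling a multicast event directly or through an OnServer relay event.
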(event `AttachPlayerOnServer`
  ;[1 1 1] AttatchPlayer to the platform (MarcoMota)
  (`self.AttachPlayerMulticast`))

(event `AttachPlayerMulticast`
  ;[1 1 1] AttatchPlayer to the platform (MarcoMota)
  (`/Game/Props/Slider/BP_U51TWMacroLibrary.AttachCharacterToMovingPlatform` (`self.Cart`) (`self.Character`)))

(event `self.ReceiveBeginPlay`
  (`|ExecutionSequence`
    (:`then_0`
      ;[1 1 1] AttatchPlayer to the platform (MarcoMota)
      (`/Engine/EditorBlueprintResources/ActorMacros.Switch Has Authority`
        (:`Authority`
          (`self.AttachPlayerMulticast`))
        (:`Remote`
          (`self.AttachPlayerOnServer`))))
    (:`then_1`
      ;[1 1 1] Set the movement/speed of the platform (MarcoMota)
      (`/Engine/EditorBlueprintResources/ActorMacros.Switch Has Authority`
        (:`Authority`
          (`self.MPSMulticast`))
        (:`Remote`
          (`self.MPSOnServer`))))))

(event `MPSOnServer`
  ;[1 1 1] Set the movement/speed of the platform (MarcoMota)
  (`self.MPSMulticast`))

(event `MPSMulticast`
  ;[1 1 1] Set the movement/speed of the platform (MarcoMota)
  (`/Game/Props/Slider/BP_U51TWMacroLibrary.MovePlatformSpline` (`self.Cart`) (`self.Spline`) 0 200.0 5 600.0
    (:`Completed`
      (`self.K2_DestroyActor` (`self.Cart`))
      (`self.K2_DestroyActor`))))

(event `self.ReceiveTick`
  (params (DeltaSeconds :type "Float (single-precision)"))
  ;[1 1 1] Update Character while platform is moving (MarcoMota)
  (`/Engine/EditorBlueprintResources/ActorMacros.Switch Has Authority`
    (:`Authority`
      (`self.UpdateCharPosMulticast`))
    (:`Remote`
      (`self.UpdateCharPosOnServer`))))

(event `UpdateCharPosMulticast`
  ;[1 1 1] Update Character while platform is moving (MarcoMota)
  (`/Game/Props/Slider/BP_U51TWMacroLibrary.UpdateCharacterPositionPlatform` (`self.Cart`) (`self.Character`)))

(event `UpdateCharPosOnServer`
  ;[1 1 1] Update Character while platform is moving (MarcoMota)
  (`self.UpdateCharPosMulticast`))

(fn `UserConstructionScript`)