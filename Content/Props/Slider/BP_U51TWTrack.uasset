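; BP_U51TWTrack is a spline track prop, optionally looped, with debug labels for its points; it has no active runtime logic.
; The Construction Script applies IsLoopable as the spline's closed-loop state inside its per-point loop, which skips the last point on open tracks.
; When DrawTrackPointNumber is on, DrawPointNumber adds a colored text component showing each index above its point, aligned to the spline and also visible in game.
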(event `self.ReceiveBeginPlay`)

(fn `DrawPointNumber`
  (params (PointIndex :type Integer))
  (bind _usefullspline (`self.UsefullSpline`))
  (bind (_returnvalue_x _returnvalue_y _returnvalue_z) (`KismetMathLibrary.BreakVector` (`SplineComponent.GetLocationAtSplinePoint` _usefullspline PointIndex "Local")))
  (if (`self.DrawTrackPointNumber`)
    (bind _returnvalue (`AddComponent|NODE_AddTextRenderComponent-1` :`RelativeTransform` (`KismetMathLibrary.MakeTransform` (`KismetMathLibrary.MakeVector` _returnvalue_x _returnvalue_y (+ _returnvalue_z 50.0)) (`SplineComponent.GetRotationAtSplinePoint` _usefullspline PointIndex "Local"))))
    (`TextRenderComponent.K2_SetText` _returnvalue (`KismetTextLibrary.Conv_IntToText` PointIndex))
    (`TextRenderComponent.SetWorldSize` _returnvalue 100.0)
    (`TextRenderComponent.SetTextRenderColor` _returnvalue (`self.TrackPointNumberColor`))
    (`SceneComponent.SetHiddenInGame` _returnvalue (not (`self.DrawTrackPointNumber`)) false)))

(fn `UserConstructionScript`
  ;[1 1 1] Create the Debug Numbers of each spline point (Marco Mota)
  (`|ExecutionSequence`
    (:`then_0`
      (set `self.NumberOfSplinePoints` (`SplineComponent.GetNumberOfSplinePoints` (`self.UsefullSpline`))))
    (:`then_1`
      (for _index (range (+ (- (`self.NumberOfSplinePoints`) (`KismetMathLibrary.SelectInt` 1 2 (`self.isLoopable?`))) 1))
        (set `self.CurrentLoopIndex` _index)
        (`SplineComponent.SetClosedLoop` (`self.UsefullSpline`) (`self.isLoopable?`) true)
        (`self.DrawPointNumber` (`self.CurrentLoopIndex`))))))