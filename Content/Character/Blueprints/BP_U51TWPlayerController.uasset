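; Player controller that gives the first player a random team, Attacker or Defender, and a random spawn location.
; On BeginPlay, it acts only when the world holds no BP_Attacker or BP_Defender actors.
; It picks one of the two classes at random, spawns it at the location of a shuffled PlayerStart and possesses it.
; It has no authority check and no handling for later players.
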(event `self.ReceiveBeginPlay`
  ;[1 1 1] Random team and spawn location for the first player, listen server or normal player (Marco Mota)
  (bind _outactors (`GameplayStatics.GetAllActorsOfClass` "/Game/Defender/Blueprints/BP_Defender.BP_Defender_C"))
  (bind _outactors_2 (`GameplayStatics.GetAllActorsOfClass` "/Game/Attacker/Blueprints/BP_Attacker.BP_Attacker_C"))
  (if (and (== (`KismetArrayLibrary.Array_Length` _outactors_2) 0) (== (`KismetArrayLibrary.Array_Length` _outactors) 0))
    (switch `int` (`KismetMathLibrary.RandomIntegerInRange` 0 1)
      (:`0`
        (bind _outactors_3 (`GameplayStatics.GetAllActorsOfClass` "/Script/Engine.PlayerStart"))
        (`KismetArrayLibrary.Array_Shuffle` _outactors_3)
        (bind _returnvalue (`|SpawnActorFromClass` "/Game/Attacker/Blueprints/BP_Attacker.BP_Attacker_C" (`KismetMathLibrary.MakeTransform` (`self.K2_GetActorLocation` (`|GetArrayItem` _outactors_3))) "Undefined" "OverrideRootScale" null "" null null))
        (`self.Possess` _returnvalue))
      (:`1`
        (bind _outactors_4 (`GameplayStatics.GetAllActorsOfClass` "/Script/Engine.PlayerStart"))
        (`KismetArrayLibrary.Array_Shuffle` _outactors_4)
        (bind _returnvalue_2 (`|SpawnActorFromClass` "/Game/Defender/Blueprints/BP_Defender.BP_Defender_C" (`KismetMathLibrary.MakeTransform` (`self.K2_GetActorLocation` (`|GetArrayItem` _outactors_4))) "Undefined" "OverrideRootScale" null "" null null))
        (`self.Possess` _returnvalue_2)))))

(fn `UserConstructionScript`)