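; BP_BaseWeapon is the base weapon Blueprint for firing, fire-mode switching and reloading.
; FireWeapon plays an animation and spawns a muzzle projectile, looping on delays for bursts and optionally decrementing local PlayerState ammo; full auto has no branch here.
; ChangeFireMode cycles through modes the DT_PersonalWeapons row supports.
; ReloadWeapon replaces or tops up the magazine per that row, writing results to the PlayerState's equipped-weapon array.
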(event `FireWeapon`
  (params (EW :type "/Game/Weapons/WeaponInfo/ST_EquipedWeapon Structure (by ref)") (PW :type "/Game/Weapons/WeaponInfo/ST_PersonalWeapons Structure (by ref)") (UpdateAmmo :type Boolean))
  (bind (_weapontype _weaponname _currentammoinmagazine _currentammoinbackpack _currentfiremode) (break `/Game/Weapons/WeaponInfo/ST_EquipedWeapon` EW))
  (bind (_weaponname_2 _weapontype_2 _weaponimage _crosshairimage _sniperscopeimage _weaponskeletalmesh _muzzleflasheffect _firesound _weaponshootinganimation _charreloadanimation _equipanimation _unequipanimation _projectile _hassingleshotmode _hasburstmode _hasfullautomode _canhaveweaponlight _hasweaponcamera _firerate _maxammoinmagazine _maxammoinbackpack _roundsinburst) (break `/Game/Weapons/WeaponInfo/ST_PersonalWeapons` PW))
  (bind _skeletalmesh (`self.SkeletalMesh`))
  ;[1 1 1] Fire (CarlosMora)
  (set `self.UpdateLocalAmmo` UpdateAmmo)
  (set `self.BurstCounter` 0)
  (`SkeletalMeshComponent.PlayAnimation` _skeletalmesh _weaponshootinganimation false :!label _label)
  (`|SpawnActorFromClass` _projectile (`SceneComponent.GetSocketTransform` _skeletalmesh "Muzzle" "RTS_World") "AlwaysSpawn" "OverrideRootScale" null null)
  (switch `/Game/Weapons/WeaponInfo/E_FireModes` _currentfiremode
    (:`NewEnumerator0`
      (`KismetSystemLibrary.Delay` _firerate)
      (if (`self.UpdateLocalAmmo`)
        (`self.UpdateAmmo`)))
    (:`NewEnumerator1`
      (`KismetSystemLibrary.Delay` (/ _firerate 2.0))
      (bind _result (`/Engine/EditorBlueprintResources/StandardMacros.IncrementInt` (`self.BurstCounter`))
        (:`  `
          (if (<= _result (`KismetMathLibrary.Min` _currentammoinmagazine _roundsinburst))
            (if (`self.UpdateLocalAmmo`)
              (`self.UpdateAmmo`)
              (goto _label)
              (else
                (goto _label)))))))))

(event `ChangeFireMode`
  (params (Player :type "PlayerState Object Reference"))
  ;[1 1 1] Retrieves weapon info from PlayerState and DataTable and changes fire mode (CarlosMora)
  (bind _asbp_u51twplayer_state (cast `/Game/Character/Blueprints/BP_U51TWPlayerState` Player))
  (bind _equipedweapons (`/Game/Character/Blueprints/BP_U51TWPlayerState.EquipedWeapons` _asbp_u51twplayer_state))
  (bind _selectedweapon (`/Game/Character/Blueprints/BP_U51TWPlayerState.SelectedWeapon` _asbp_u51twplayer_state))
  (bind (_weapontype _weaponname _currentammoinmagazine _currentammoinbackpack _currentfiremode _currentweaponstate _currentweaponlight) (break `/Game/Weapons/WeaponInfo/ST_EquipedWeapon` (`|GetArrayItem` _equipedweapons _selectedweapon)))
  (set `self.FireMode` _currentfiremode)
  (bind _returnvalue (`|GetDataTableRow` "/Game/Weapons/WeaponInfo/DT_PersonalWeapons.DT_PersonalWeapons" _weaponname)
    (:`then`
      (switch `/Game/Weapons/WeaponInfo/E_FireModes` (`self.FireMode`)
        (:`NewEnumerator0`
          (bind (_weaponname_2 _weapontype_2 _weaponimage _crosshairimage _sniperscopeimage _weaponskeletalmesh _muzzleflasheffect _firesound _weaponshootinganimation _charreloadanimation _equipanimation _unequipanimation _projectile _hassingleshotmode _hasburstmode _hasfullautomode) (break `/Game/Weapons/WeaponInfo/ST_PersonalWeapons` _returnvalue))
          (if _hasburstmode :!label _label_2
            (set `self.FireMode` "NewEnumerator1")
            (else
              (if _hasfullautomode :!label _label_3
                (set `self.FireMode` "NewEnumerator2")
                (else
                  (if _hassingleshotmode :!label _label_4
                    (set `self.FireMode` "NewEnumerator0")
                    (else
                      (goto _label_2))))))))
        (:`NewEnumerator1`
          (goto _label_3))
        (:`NewEnumerator2`
          (goto _label_4)))
      (`KismetArrayLibrary.Array_Set` _equipedweapons _selectedweapon (make `/Game/Weapons/WeaponInfo/ST_EquipedWeapon` _weapontype _weaponname _currentammoinmagazine _currentammoinbackpack (`self.FireMode`) _currentweaponstate _currentweaponlight)))))

(event `ReloadWeapon`
  (params (Player :type "PlayerState Object Reference"))
  ;[1 1 1] Retrieves weapon info from PlayerState and DataTable and reloads weapon (CarlosMora)
  (bind _asbp_u51twplayer_state (cast `/Game/Character/Blueprints/BP_U51TWPlayerState` Player))
  (bind _equipedweapons (`/Game/Character/Blueprints/BP_U51TWPlayerState.EquipedWeapons` _asbp_u51twplayer_state))
  (bind _selectedweapon (`/Game/Character/Blueprints/BP_U51TWPlayerState.SelectedWeapon` _asbp_u51twplayer_state))
  (bind (_weapontype _weaponname _currentammoinmagazine _currentammoinbackpack _currentfiremode _currentweaponstate _currentweaponlight) (break `/Game/Weapons/WeaponInfo/ST_EquipedWeapon` (`|GetArrayItem` _equipedweapons _selectedweapon)))
  (if (>= _currentammoinbackpack 0)
    (bind _returnvalue (`|GetDataTableRow` "/Game/Weapons/WeaponInfo/DT_PersonalWeapons.DT_PersonalWeapons" _weaponname)
      (:`then`
        (bind (_weaponname_2 _weapontype_2 _weaponimage _crosshairimage _sniperscopeimage _weaponskeletalmesh _muzzleflasheffect _firesound _weaponshootinganimation _charreloadanimation _equipanimation _unequipanimation _projectile _hassingleshotmode _hasburstmode _hasfullautomode _canhaveweaponlight _hasweaponcamera _firerate _maxammoinmagazine _maxammoinbackpack _roundsinburst _projectile_maxdamage _projectile_mindamage _projectile_speed _autoreload _consumeallroundsonreload) (break `/Game/Weapons/WeaponInfo/ST_PersonalWeapons` _returnvalue))
        (if _consumeallroundsonreload
          ;;[1 1 1] Reload replaces magazine
          (if (>= _currentammoinbackpack _maxammoinmagazine)
            (bind _output_get (set `self.TransferedAmmo` _maxammoinmagazine))
            (set `self.UpdatedAmmo` _output_get)
            (else
              (bind _output_get_2 (set `self.TransferedAmmo` _currentammoinbackpack))
              (set `self.UpdatedAmmo` _output_get_2)))
          (`KismetArrayLibrary.Array_Set` _equipedweapons _selectedweapon (make `/Game/Weapons/WeaponInfo/ST_EquipedWeapon` _weapontype _weaponname (`self.UpdatedAmmo`) (- _currentammoinbackpack (`self.TransferedAmmo`)) _currentfiremode _currentweaponstate _currentweaponlight) :!label _label_5)
          (else
            ;;[1 1 1] Reload fills magazine
            (if (> _currentammoinbackpack 0)
              (bind _output_get_3 (set `self.TransferedAmmo` (`KismetMathLibrary.Abs_Int` (- (`KismetMathLibrary.Min` _maxammoinmagazine _currentammoinbackpack) _currentammoinmagazine))))
              (set `self.UpdatedAmmo` (+ _output_get_3 _currentammoinmagazine))
              (goto _label_5))))))))

(fn `UpdateAmmo`
  ;[1 1 1] Get local PlayerState and updates ammo of selected weapon (only runs on client requesting the fire shot) (CarlosMora)
  (bind _asbp_u51twplayer_state (cast `/Game/Character/Blueprints/BP_U51TWPlayerState` (`Controller.PlayerState` (`GameplayStatics.GetPlayerController` 0))))
  (bind _equipedweapons (`/Game/Character/Blueprints/BP_U51TWPlayerState.EquipedWeapons` _asbp_u51twplayer_state))
  (bind _selectedweapon (`/Game/Character/Blueprints/BP_U51TWPlayerState.SelectedWeapon` _asbp_u51twplayer_state))
  (bind (_weapontype _weaponname _currentammoinmagazine _currentammoinbackpack _currentfiremode _currentweaponstate _currentweaponlight) (break `/Game/Weapons/WeaponInfo/ST_EquipedWeapon` (`|GetArrayItem` _equipedweapons _selectedweapon)))
  (`KismetArrayLibrary.Array_Set` _equipedweapons _selectedweapon (make `/Game/Weapons/WeaponInfo/ST_EquipedWeapon` _weapontype _weaponname (- _currentammoinmagazine 1) _currentammoinbackpack _currentfiremode _currentweaponstate _currentweaponlight)))

(fn `UserConstructionScript`)